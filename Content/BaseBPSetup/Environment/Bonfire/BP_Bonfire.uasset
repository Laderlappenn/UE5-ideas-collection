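; BP_Bonfire is an environment bonfire actor with a flickering point light and proximity-triggered sound.
; On BeginPlay, a timeline at raised play rate drives the light intensity between minimum and maximum values through a Lerp.
; Any actor overlap adds and stores an audio component, and end overlap destroys the stored one.
; A looping timer setup bound to an empty Timeline event is never executed.
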(event `Timeline`)

(event `self.ReceiveBeginPlay`
  (`TimelineComponent.SetPlayRate` (`self.TM_LightFlickering`) 2.0)
  (bind (_direction _alpha) (`Timeline|TM_LightFlickering`)
    (:`Update`
      (`LightComponent.SetIntensity` (`self.PointLight`) (`KismetMathLibrary.Lerp` (`self.MinIntensity`) (`self.MaxIntensity`) _alpha)))))

(event `self.ReceiveActorBeginOverlap`
  (params (OtherActor :type "Actor Object Reference"))
  (bind _returnvalue (`AddComponent|NODE_AddAudioComponent-0`))
  (set `self.BonfireSound` _returnvalue))

(event `self.ReceiveActorEndOverlap`
  (params (OtherActor :type "Actor Object Reference"))
  (bind _bonfiresound (`self.BonfireSound`)
    (:`then`
      (`ActorComponent.K2_DestroyComponent` _bonfiresound))
    (:`else`)))

(fn `UserConstructionScript`)