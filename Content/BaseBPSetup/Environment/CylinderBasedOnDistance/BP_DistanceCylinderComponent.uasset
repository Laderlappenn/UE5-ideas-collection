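; Environment cylinder actor that changes its height according to the player character's horizontal proximity.
; On BeginPlay it derives an end location by offsetting its start position down by Distance.
; Each tick it maps player distance to a clamped factor that scales the end location's world Z, reaching that lowered position when the player is close.
; Scaling absolute Z, rather than interpolating from the start location, makes the motion depend on world height.
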(event `self.ReceiveBeginPlay`
  (set `self.StartLocation` (`self.K2_GetActorLocation`))
  (set `self.EndLocation` (+ (`self.StartLocation`) (`KismetMathLibrary.MakeVector` 0.0 0.0 (* (`self.Distance`) -1.0)))))

(event `self.ReceiveTick`
  (params (DeltaSeconds :type "Float (single-precision)"))
  (bind (_endlocation_x _endlocation_y _endlocation_z) (`KismetMathLibrary.BreakVector` (`self.EndLocation`)))
  (`/Engine/EditorBlueprintResources/StandardMacros.IsValid` (`GameplayStatics.GetPlayerCharacter` 0)
    (:`Is Valid`
      (`self.K2_SetActorLocation` (`KismetMathLibrary.MakeVector` _endlocation_x _endlocation_y (* _endlocation_z (`KismetMathLibrary.MapRangeClamped` (`self.GetHorizontalDistanceTo` (`GameplayStatics.GetPlayerCharacter` 0) self) 100.0 500.0 1.0)))))))

(fn `UserConstructionScript`)