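; BP_CylinderComponent is a moving cylinder environment actor that travels vertically from its placed location to a point Distance units below it.
; On BeginPlay it caches both endpoints and briefly draws colored debug spheres at them.
; It then plays the TM_Moving timeline, whose Alpha lerps the actor between the endpoints without sweep or teleport.
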(event `self.ReceiveBeginPlay`
  (set `self.StartLocation` (`self.K2_GetActorLocation`))
  (set `self.EndLocation` (+ (`self.StartLocation`) (`KismetMathLibrary.MakeVector` 0.0 0.0 (* (`self.Distance`) -1.0))))
  (`KismetSystemLibrary.DrawDebugSphere` (`self.StartLocation`) 55.0 12 (struct :`R` 0.214954 :`G` 1.0 :`A` 1.0) 5.0)
  (`KismetSystemLibrary.DrawDebugSphere` (`self.EndLocation`) 55.0 12 (struct :`R` 1.0 :`G` 0.153681 :`A` 1.0) 5.0)
  (bind (_direction _alpha) (`Timeline|TM_Moving`)
    (:`Update`
      (`self.K2_SetActorLocation` (`KismetMathLibrary.VLerp` (`self.StartLocation`) (`self.EndLocation`) _alpha)))))

(fn `UserConstructionScript`)