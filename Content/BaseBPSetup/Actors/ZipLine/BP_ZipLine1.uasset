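; BP_ZipLine1 is a zipline actor that tethers the player character with a visible cable and a physics constraint.
; When the player enters CollisionSphere, the Cable is shown with its end attached to the player, and the PhysicsConstraint links EnvironmentSphere to the player's capsule.
; Leaving the sphere detaches and hides the cable but does not break the constraint.
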(event `self.CollisionSphere.OnComponentBeginOverlap`
  (params (OverlappedComponent :type "PrimitiveComponent Object Reference") (OtherActor :type "Actor Object Reference") (OtherComp :type "PrimitiveComponent Object Reference") (OtherBodyIndex :type Integer) (bFromSweep :type Boolean) (SweepResult :type "HitResult Structure (by ref)"))
  (if (== OtherActor (`GameplayStatics.GetPlayerCharacter` 0))
    (set `CableComponent.bAttachEnd` true (`self.Cable`))
    (`SceneComponent.SetHiddenInGame` (`self.Cable`) false false)
    (`CableComponent.SetAttachEndTo` (`self.Cable`) (`GameplayStatics.GetPlayerCharacter` 0) "None" "None")
    (`PhysicsConstraintComponent.SetConstrainedComponents` (`self.PhysicsConstraint`) (`self.EnvironmentSphere`) "None" (`Character.CapsuleComponent` (`GameplayStatics.GetPlayerCharacter` 0)) "None")))

(event `self.CollisionSphere.OnComponentEndOverlap`
  (params (OverlappedComponent :type "PrimitiveComponent Object Reference") (OtherActor :type "Actor Object Reference") (OtherComp :type "PrimitiveComponent Object Reference") (OtherBodyIndex :type Integer))
  (if (== OtherActor (`GameplayStatics.GetPlayerCharacter` 0))
    (set `CableComponent.bAttachEnd` false (`self.Cable`))
    (`SceneComponent.SetHiddenInGame` (`self.Cable`) true false)))

(fn `UserConstructionScript`)