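; BP_CannonGun is a mannable cannon that takes over input and camera when the top-down character overlaps it, returning both on E.
; Looping timers drive WASD aiming, yawing the actor and pitching a gun component while keys are held.
; Left click spawns a BP_CannonProjectile and launches it by impulse along the trunk's right vector.
; Right click draws a predicted path using a velocity approximated by dividing the impulse by a hardcoded constant.
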(event `self.EnterCollision.OnComponentBeginOverlap`
  (params (OverlappedComponent :type "PrimitiveComponent Object Reference") (OtherActor :type "Actor Object Reference") (OtherComp :type "PrimitiveComponent Object Reference") (OtherBodyIndex :type Integer) (bFromSweep :type Boolean) (SweepResult :type "HitResult Structure (by ref)"))
  (bind _asbp_top_down_character (cast `/Game/TopDown/Blueprints/BP_TopDownCharacter` OtherActor))
  (set `self.As BP Top Down Character` _asbp_top_down_character)
  (bind _asbp_top_down_controller (cast `/Game/TopDown/Blueprints/BP_TopDownController` (`Pawn.GetController` (`self.As BP Top Down Character`))))
  (set `self.As BP Top Down Controller` _asbp_top_down_controller)
  (`self.DisableInput` (`self.As BP Top Down Character`) (`self.As BP Top Down Controller`))
  (`self.EnableInput` (`self.As BP Top Down Controller`))
  (`PlayerController.SetViewTargetWithBlend` (`self.As BP Top Down Controller`) self 1.0 "VTBlend_Linear" 0.0 false))

(event `Key|A`
  (params (Key :type "Key Structure"))
  (:`Pressed`
    (bind _returnvalue (`KismetSystemLibrary.K2_SetTimerDelegate` (delegate `RotationLeft`) (`self.RotationTime`) true))
    (set `self.TH_RotationLeft` _returnvalue))
  (:`Released`
    (`KismetSystemLibrary.K2_ClearAndInvalidateTimerHandle` (`self.TH_RotationLeft`))))

(event `RotationLeft`
  (`self.K2_AddActorWorldRotation` (struct :`Yaw` -1.0)))

(event `Key|D`
  (params (Key :type "Key Structure"))
  (:`Pressed`
    (bind _returnvalue (`KismetSystemLibrary.K2_SetTimerDelegate` (delegate `RotationRight`) (`self.RotationTime`) true))
    (set `self.TH_RotationRight` _returnvalue))
  (:`Released`
    (`KismetSystemLibrary.K2_ClearAndInvalidateTimerHandle` (`self.TH_RotationRight`))))

(event `RotationRight`
  (`self.K2_AddActorWorldRotation` (struct :`Yaw` 1.0)))

(event `Key|LeftMouseButton`
  (params (Key :type "Key Structure"))
  (bind _guntrunk (`self.GunTrunk`))
  (bind _returnvalue (`SceneComponent.K2_GetComponentLocation` _guntrunk))
  (bind _returnvalue_location (`KismetMathLibrary.BreakTransform` (`SceneComponent.K2_GetComponentToWorld` (`self.GunTrunk`))))
  (bind _returnvalue_2 (`SceneComponent.GetRightVector` _guntrunk))
  (:`Pressed`
    (bind _returnvalue_3 (`|SpawnActorFromClass` "/Game/BaseBPSetup/Actors/CannonGun/BP_CannonProjectile.BP_CannonProjectile_C" (`KismetMathLibrary.MakeTransform` _returnvalue_location (`KismetMathLibrary.Conv_VectorToRotator` (`SceneComponent.GetRightVector` (`self.GunTrunk`)))) "Undefined" "MultiplyWithRoot" null null))
    ;[1 1 1] may be shooting logic better to implement inside BP_CannonProjectile with Projectile Movement Component
    (bind _output_get (set `self.Projectile` _returnvalue_3))
    (`PrimitiveComponent.AddImpulseAtLocation` (`/Game/BaseBPSetup/Actors/CannonGun/BP_CannonProjectile.ProjectileSphere` _output_get) (* _returnvalue_2 (`self.ImpulseMultiplier `)) _returnvalue "None")
    (`KismetSystemLibrary.DrawDebugArrow` _returnvalue (+ _returnvalue (* _returnvalue_2 200.0)) 5.0 (struct :`R` 0.148108 :`G` 1.0 :`A` 1.0) 2.0 2.0)))

(event `Key|RightMouseButton`
  (params (Key :type "Key Structure"))
  (:`Pressed`
    (`GameplayStatics.Blueprint_PredictProjectilePath_ByTraceChannel` (`SceneComponent.K2_GetComponentLocation` (`self.GunTrunk`)) (`self.GetLaunchVelocity(Bad)`) true 20.0 "ECC_WorldStatic" false (`|MakeArray` self (`|GetArrayItem` (`PrimitiveComponent.GetOverlappingActors` (`self.GunTrunk`) "/Game/BaseBPSetup/Actors/CannonGun/BP_CannonProjectile.BP_CannonProjectile_C")) :!type "Actor Object Reference") "ForDuration" 5.0 10.0 1.0)))

(event `Key|E`
  (params (Key :type "Key Structure"))
  (:`Pressed`
    (`self.DisableInput` (`self.As BP Top Down Controller`))
    (`self.EnableInput` (`self.As BP Top Down Character`) (`self.As BP Top Down Controller`))
    (`PlayerController.SetViewTargetWithBlend` (`self.As BP Top Down Controller`) (`self.As BP Top Down Character`) 1.0 "VTBlend_Linear" 0.0 false)))

(event `Key|W`
  (params (Key :type "Key Structure"))
  (:`Pressed`
    (bind _returnvalue (`KismetSystemLibrary.K2_SetTimerDelegate` (delegate `RotationUp`) (`self.RotationTime`) true))
    (set `self.TH_RotationUp` _returnvalue))
  (:`Released`
    (`KismetSystemLibrary.K2_ClearAndInvalidateTimerHandle` (`self.TH_RotationUp`))))

(event `RotationUp`
  (`SceneComponent.K2_AddRelativeRotation` (`self.Cube8`) (struct :`Roll` 1.0) false false))

(event `Key|S`
  (params (Key :type "Key Structure"))
  (:`Pressed`
    (bind _returnvalue (`KismetSystemLibrary.K2_SetTimerDelegate` (delegate `RotationDown`) (`self.RotationTime`) true))
    (set `self.TH_RotationDown` _returnvalue))
  (:`Released`
    (`KismetSystemLibrary.K2_ClearAndInvalidateTimerHandle` (`self.TH_RotationDown`))))

(event `RotationDown`
  (`SceneComponent.K2_AddRelativeRotation` (`self.Cube8`) (struct :`Roll` -1.0) false false))

(fn `GetLaunchVelocity(Bad)`
  (returns (ReturnValue :type "Vector Structure"))
  (return (* (`SceneComponent.GetRightVector` (`self.GunTrunk`)) (/ (`KismetMathLibrary.Conv_IntToDouble` (`self.ImpulseMultiplier `)) 24.2))))

(fn `UserConstructionScript`)