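; BP_CannonProjectile is a cannon projectile actor that destroys itself five seconds after it begins play.
; While any ProjectileSphere rigid body is awake, Tick predicts a short path from the sphere's current location and velocity, tracing against WorldStatic.
; The prediction serves only as a one-frame debug drawing, as its result is not used.
; The ProjectileMovement component is not used by the graph.
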(event `self.ReceiveBeginPlay`
  (`KismetSystemLibrary.Delay` 5.0)
  (`self.K2_DestroyActor`))

(event `self.ReceiveTick`
  (params (DeltaSeconds :type "Float (single-precision)"))
  (if (`PrimitiveComponent.IsAnyRigidBodyAwake` (`self.ProjectileSphere`))
    (`GameplayStatics.Blueprint_PredictProjectilePath_ByTraceChannel` (`self.K2_GetActorLocation`) (`SceneComponent.GetComponentVelocity` (`self.ProjectileSphere`)) true 20.0 "ECC_WorldStatic" false (`|MakeArray` self :!type "Actor Object Reference") "ForOneFrame" 1.0 5.0 1.0)))

(fn `UserConstructionScript`)