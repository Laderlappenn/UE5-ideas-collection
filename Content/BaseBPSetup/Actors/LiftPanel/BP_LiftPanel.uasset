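; Lift platform actor that travels a set vertical distance, up or down, when the player character steps on it.
; Two timelines lerp between start and end locations, with play rate derived from a travel time.
; After a delay at the end, it returns once the player is off.
; An underside trigger pauses only the outbound timeline while overlapped, and debug spheres mark both endpoints at BeginPlay.
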(event `self.ReceiveBeginPlay`
  (set `self.StartLocation` (`self.K2_GetActorLocation`))
  (set `self.EndLocation` (+ (`self.StartLocation`) (`KismetMathLibrary.MakeVector` 0.0 0.0 (* (`self.Distance`) (`KismetMathLibrary.SelectFloat` 1.0 -1.0 (`self.Up / Down`))))))
  (`KismetSystemLibrary.DrawDebugSphere` (`self.StartLocation`) 25.0 12 (struct :`R` 0.214954 :`G` 1.0 :`A` 1.0) 5.0)
  (`KismetSystemLibrary.DrawDebugSphere` (`self.EndLocation`) 25.0 12 (struct :`R` 1.0 :`G` 0.153681 :`A` 1.0) 5.0))

(event `self.Box.OnComponentBeginOverlap`
  (params (OverlappedComponent :type "PrimitiveComponent Object Reference") (OtherActor :type "Actor Object Reference") (OtherComp :type "PrimitiveComponent Object Reference") (OtherBodyIndex :type Integer) (bFromSweep :type Boolean) (SweepResult :type "HitResult Structure (by ref)"))
  (if (== OtherActor (`GameplayStatics.GetPlayerCharacter` 0))
    (set `self.IsCharacterOnPlatform` true)
    (if (`self.CanLift`)
      (set `self.CanLift` false)
      (set `self.CanLiftOnEndOverlap` false)
      (`TimelineComponent.SetPlayRate` (`self.TM_Begin`) (/ 1.0 (`self.MoveUpTimeInSeconds`)))
      (bind (_direction _alpha) (`Timeline|TM_Begin` :!via `PlayFromStart`)
        (:`Update`
          (`self.K2_SetActorLocation` (`KismetMathLibrary.VLerp` (`self.StartLocation`) (`self.EndLocation`) _alpha)))
        (:`Finished`
          (`KismetSystemLibrary.Delay` (`self.TimeToLiftToStart`))
          (if (`self.IsCharacterOnPlatform`)
            (set `self.CanLiftOnEndOverlap` true)
            (set `self.CanLift` true)
            (else
              (`self.MoveToStart`))))))))

(event `self.Box.OnComponentEndOverlap`
  (params (OverlappedComponent :type "PrimitiveComponent Object Reference") (OtherActor :type "Actor Object Reference") (OtherComp :type "PrimitiveComponent Object Reference") (OtherBodyIndex :type Integer))
  (if (== OtherActor (`GameplayStatics.GetPlayerCharacter` 0))
    (set `self.IsCharacterOnPlatform` false)
    (if (`self.CanLiftOnEndOverlap`)
      (if (`self.CanLift`)
        (`self.MoveToStart`)))))

(event `MoveToStart`
  (set `self.CanLift` false)
  (`TimelineComponent.SetPlayRate` (`self.TM_End`) (/ 1.0 (`self.MoveUpTimeInSeconds`)))
  (bind (_direction _alpha) (`Timeline|TM_End` :!via `PlayFromStart`)
    (:`Update`
      (`self.K2_SetActorLocation` (`KismetMathLibrary.VLerp` (`self.EndLocation`) (`self.StartLocation`) _alpha)))
    (:`Finished`
      (set `self.CanLift` true))))

(event `self.PreventCollidingUnderPlatform.OnComponentBeginOverlap`
  (params (OverlappedComponent :type "PrimitiveComponent Object Reference") (OtherActor :type "Actor Object Reference") (OtherComp :type "PrimitiveComponent Object Reference") (OtherBodyIndex :type Integer) (bFromSweep :type Boolean) (SweepResult :type "HitResult Structure (by ref)"))
  (`TimelineComponent.Stop` (`self.TM_Begin`)))

(event `self.PreventCollidingUnderPlatform.OnComponentEndOverlap`
  (params (OverlappedComponent :type "PrimitiveComponent Object Reference") (OtherActor :type "Actor Object Reference") (OtherComp :type "PrimitiveComponent Object Reference") (OtherBodyIndex :type Integer))
  (`TimelineComponent.Play` (`self.TM_Begin`)))

(fn `UserConstructionScript`)