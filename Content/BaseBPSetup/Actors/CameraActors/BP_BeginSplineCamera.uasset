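; Intro camera actor that, when BeginCameraIntro is set, takes over the player's view at BeginPlay and flies along a spline.
; A slowed timeline drives the camera by distance along the spline, aiming it along the tangent (read in local space, applied as world rotation).
; When the timeline finishes, SplineEnd blends the view back to the player character.
; The construction script places the camera at the first spline point.
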(event `self.ReceiveBeginPlay`
  (if (`self.BeginCameraIntro`)
    (`TimelineComponent.SetPlayRate` (`self.TM_SmoothCameraOnSplline`) 0.2)
    (`PlayerController.SetViewTargetWithBlend` (`GameplayStatics.GetPlayerController` 0) self 0.0 "VTBlend_Linear" 0.0 false)
    (bind (_direction _alpha) (`Timeline|TM_SmoothCameraOnSplline` :!via `PlayFromStart`)
      (:`Update`
        (bind _returnvalue (`KismetMathLibrary.Lerp` 0.0 (`SplineComponent.GetDistanceAlongSplineAtSplinePoint` (`self.Spline`) (- (`SplineComponent.GetNumberOfSplinePoints` (`self.Spline`)) 1)) _alpha))
        (`SceneComponent.K2_SetWorldLocation` (`self.Camera`) (`SplineComponent.GetLocationAtDistanceAlongSpline` (`self.Spline`) _returnvalue "World") false false)
        (`SceneComponent.K2_SetWorldRotation` (`self.Camera`) (`KismetMathLibrary.Conv_VectorToRotator` (`SplineComponent.GetTangentAtDistanceAlongSpline` (`self.Spline`) _returnvalue "Local")) false false))
      (:`Finished`
        (`self.SplineEnd`)))))

(event `SplineEnd`
  (`PlayerController.SetViewTargetWithBlend` (`GameplayStatics.GetPlayerController` 0) (`GameplayStatics.GetPlayerCharacter` 0) 3.0 "VTBlend_Linear" 0.0 false))

(fn `UserConstructionScript`
  (`SceneComponent.K2_SetWorldLocation` (`self.Camera`) (`SplineComponent.GetLocationAtSplinePoint` (`self.Spline`) 0 "World") false false))